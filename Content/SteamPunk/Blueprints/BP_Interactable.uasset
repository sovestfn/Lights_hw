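; BP_Interactable is an interactable actor that shows a widget prompt facing the player's camera.
; BeginPlay caches the player's third-person character, and TurnonInteract and TurnOffInteract show or hide the widget while starting or clearing a looping timer.
; RotateWiget turns the widget toward the follow camera using only X and Y, so it yaws without tilting, apparently driven by that timer instead of Tick.
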(event `self.ReceiveBeginPlay`
  (bind _asbp_third_person_character (cast `/Game/ThirdPerson/Blueprints/BP_ThirdPersonCharacter` (`GameplayStatics.GetPlayerPawn` 0)))
  (set `self.As BP Third Person Character` _asbp_third_person_character))

(event `/Game/SteamPunk/BPI_Interactable.TurnOnInteract`
  (`SceneComponent.SetHiddenInGame` (`self.Widget`) false true)
  (bind _returnvalue (`KismetSystemLibrary.K2_SetTimerDelegate` (`|CreateDelegate` :!event `RotateWiget`) 0.04 true))
  (set `self.TimerHandler` _returnvalue))

(event `/Game/SteamPunk/BPI_Interactable.TurnOffInteract`
  (`SceneComponent.SetHiddenInGame` (`self.Widget`) true true)
  (`KismetSystemLibrary.K2_ClearAndInvalidateTimerHandle` (`self.TimerHandler`)))

(event `RotateWiget`
  (bind _widget (`self.Widget`))
  (bind (_returnvalue_x _returnvalue_y) (`KismetMathLibrary.BreakVector` (`SceneComponent.K2_GetComponentLocation` _widget)))
  (bind (_returnvalue_x_2 _returnvalue_y_2) (`KismetMathLibrary.BreakVector` (`SceneComponent.K2_GetComponentLocation` (`/Game/ThirdPerson/Blueprints/BP_ThirdPersonCharacter.FollowCamera` (`self.As BP Third Person Character`)))))
  (`SceneComponent.K2_SetWorldRotation` _widget (`KismetMathLibrary.FindLookAtRotation` (`KismetMathLibrary.MakeVector` _returnvalue_x _returnvalue_y) (`KismetMathLibrary.MakeVector` _returnvalue_x_2 _returnvalue_y_2)) false false))

(fn `UserConstructionScript`)