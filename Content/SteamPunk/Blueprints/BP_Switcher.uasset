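; BP_Switcher is an interactable lever switch that turns an assigned set of lights on and off.
; Each InteractAction flips between two states, rotating the handle to its default or to a -90 degree roll.
; It then loops over the Lights array and sends on or off messages through BPI_Lights to actors that implement it.
; Begin and end overlap events simply defer to the parent class.
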(event `self.ReceiveActorBeginOverlap`
  (params (OtherActor :type "Actor Object Reference"))
  (`parent.ReceiveActorBeginOverlap` OtherActor))

(event `self.ReceiveActorEndOverlap`
  (params (OtherActor :type "Actor Object Reference"))
  (`parent.ReceiveActorEndOverlap` OtherActor))

(event `/Game/SteamPunk/BPI_Interactable.InteractAction`
  (`/Engine/EditorBlueprintResources/StandardMacros.FlipFlop`
    (:`A`
      (`SceneComponent.K2_SetRelativeRotation` (`self.switchHandler_handler`) (`KismetMathLibrary.MakeRotator` 0.0) false false)
      (for _array_element (`self.Lights`)
        (if (`KismetSystemLibrary.DoesImplementInterface` _array_element "/Game/SteamPunk/BPI_Lights.BPI_Lights_C")
          (message `/Game/SteamPunk/BPI_Lights.TurnOnLight` _array_element))))
    (:`B`
      (`SceneComponent.K2_SetRelativeRotation` (`self.switchHandler_handler`) (`KismetMathLibrary.MakeRotator` -90.0) false false)
      (for _array_element_2 (`self.Lights`)
        (if (`KismetSystemLibrary.DoesImplementInterface` _array_element_2 "/Game/SteamPunk/BPI_Lights.BPI_Lights_C")
          (message `/Game/SteamPunk/BPI_Lights.TurnOffLight` _array_element_2))))))

(fn `UserConstructionScript`)