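; Main light switch that, on Interact, tilts its switch mesh between two positions and toggles the lights it controls.
; Each entry in the Lights array that implements BPI_Lights receives SwitchLightMessage.
; Inside that same loop, an apparently experimental step finds all DirectionalLights and sets their visibility from a FlipFlop, which alternates on every iteration rather than once per press.
; Overlap events only forward to the parent.
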(event `self.ReceiveActorBeginOverlap`
  (params (OtherActor :type "Actor Object Reference"))
  (`parent.ReceiveActorBeginOverlap` OtherActor))

(event `self.ReceiveActorEndOverlap`
  (params (OtherActor :type "Actor Object Reference"))
  (`parent.ReceiveActorEndOverlap` OtherActor))

(event `/Game/SteamPunk/Interfaces/BPI_Interactable.Interact`
  (`/Engine/EditorBlueprintResources/StandardMacros.FlipFlop`
    (:`A`
      (`SceneComponent.K2_SetRelativeRotation` (`self.lightswitch_Switch_001`) (`KismetMathLibrary.MakeRotator` 0.0 -8.0 90.0) false false))
    (:`B`
      (`SceneComponent.K2_SetRelativeRotation` (`self.lightswitch_Switch_001`) (`KismetMathLibrary.MakeRotator` 0.0 0.0 90.0) false false)))
  (for _array_element (`self.Lights`)
    (if (`KismetSystemLibrary.DoesImplementInterface` _array_element "/Game/SteamPunk/Interfaces/BPI_Lights.BPI_Lights_C")
      (message `/Game/SteamPunk/Interfaces/BPI_Lights.SwitchLight` _array_element)
      ;[1 1 1] Попробовала)
      (bind _outactors (`GameplayStatics.GetAllActorsOfClass` "/Script/Engine.DirectionalLight"))
      (for _array_element_2 _outactors
        (bind _isa (`/Engine/EditorBlueprintResources/StandardMacros.FlipFlop`)
          (:`A`
            _)
          (:`B`
            _))
        (`SceneComponent.SetVisibility` (`Light.LightComponent` _array_element_2) _isa false)))))

(fn `UserConstructionScript`)